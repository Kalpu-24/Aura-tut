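; Arcane Shards gameplay ability that places a set of ground points at a mouse-targeted spot, currently only visualized with debug spheres.
; On activation it shows the avatar's magic circle and waits for an input press to capture target data under the mouse.
; A temporary BP_PointCollection spawned at the impact computes the points with random yaw.
; The ability then hides the circle, destroys the collection after a short delay and ends.
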(event Ability|EventActivateAbility
  (Utilities|FlowControl|Sequence
    (:then_0
      (Class|PlayerInterface|ShowMagicCircle(Message) (Ability|GetAvatarActorfromActorInfo) 0))
    (:then_1
      (Ability|Tasks|WaitInputPress false
        (:OnPress
          (bind _datahandle (|TargetDataUnderMouse)
            (:ValidData
              (bind _returnvalue (Game|SpawnActorfromClass "/Game/Blueprints/AbilitySystem/Aura/Abilities/Arcane/ArcaneShards/BP_PointCollection.BP_PointCollection_C" (Math|Transform|MakeTransform (.ImpactPoint (Collision|BreakHitResult (Ability|TargetData|GetHitResultfromTargetData _datahandle))) "0, 0, 0" "1.000000,1.000000,1.000000") "AlwaysSpawn" "MultiplyWithRoot" 0 0))
              (Variables|Default|SetPointCollection _returnvalue)
              (bind _output_get (Variables|Default|SetGroundPoints (Class|PointCollection|GetGroundPoints _returnvalue (.ImpactPoint (Collision|BreakHitResult (Ability|TargetData|GetHitResultfromTargetData _datahandle))) 11 (Math|Random|RandomFloatinRange 0.0 3.6e+02))))
              (for _array_element _output_get
                (Rendering|Debug|DrawDebugSphere (Transformation|GetWorldLocation _array_element) 2e+01 12 "(R=1.000000,G=1.000000,B=1.000000,A=1.000000)" 2e+01))
              (Class|PlayerInterface|HideMagicCircle(Message) (Ability|GetAvatarActorfromActorInfo))
              (Utilities|FlowControl|Delay 0.2)
              (Actor|DestroyActor (Variables|Default|GetPointCollection))
              (Ability|EndAbility))))))))

(event Ability|EventOnEndAbility
  (params (bWasCancelled :type Boolean)))