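; Aura's Fire Blast fireball actor, which flies out along its forward vector and then returns to its instigator like a boomerang.
; On the authority only, an Outgoing timeline lerps it to an apex at TravelDistance, then a Returning timeline lerps it toward the instigator's current location.
; Each return update checks ExplodeDistance to the instigator and, once within range, calls OnHit and destroys the actor.
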(event EventStartOutgoingTimeline
  (Networking|SwitchHasAuthority
    (:Authority
      (bind _output_get (Variables|Default|SetInitial%20Location (Transformation|GetActorLocation)))
      (Variables|Default|SetApexLocation (+ _output_get (* (Transformation|GetActorForwardVector) (Variables|Default|GetTravelDistance))))
      (bind _outgoingtrack (Timeline|Outgoing Play)
        (:Update
          (Transformation|SetActorLocation (Math|Vector|Lerp(Vector) (Variables|Default|GetInitial%20Location) (Variables|Default|GetApexLocation) _outgoingtrack) false false))
        (:Finished
          (bind _returningtrack (Timeline|Returning Play)
            (:Update
              (Transformation|SetActorLocation (Math|Vector|Lerp(Vector) (Variables|Default|GetApexLocation) (Transformation|GetActorLocation (Variables|Default|GetInstigator)) _returningtrack) false false)
              (if (CallFunction|IsWithinExplodeDistance)
                (Class|AuraProjectile|OnHit)
                (Actor|DestroyActor)))))))))

(fn ConstructionScript)

(fn IsWithinExplodeDistance
  (return (<= (Math|Vector|VectorLength (- (Transformation|GetActorLocation) (Transformation|GetActorLocation (Variables|Default|GetInstigator)))) (Variables|Default|GetExplodeDistance))))