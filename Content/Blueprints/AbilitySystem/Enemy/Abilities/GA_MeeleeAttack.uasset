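; Enemy melee gameplay ability that warps the avatar toward its combat target and plays a random tagged attack montage.
; The montage's gameplay event triggers a small sphere query at the matching combat socket, damaging live non-friendly players found.
; The melee impact gameplay cue then fires and the ability ends, without stopping the montage.
; Montage completion, interruption or cancellation also leads to the cue and ability end.
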(event Ability|EventActivateAbility
  (bind _returnvalue (Ability|GetAvatarActorfromActorInfo))
  (bind _returnvalue_2 (Ability|GetAvatarActorfromActorInfo))
  (bind _returnvalue_3 (Class|TargetInterface|GetCombatTarget(Message) _returnvalue))
  (Class|CombatInterface|UpdateRotationMotionWarp(Message) _returnvalue (Transformation|GetActorLocation _returnvalue_3))
  (bind _returnvalue_4 (Class|CombatInterface|GetAttackMontages(Message) _returnvalue))
  (bind (_montage _montagetag) (CallFunction|GetRandomAttackMontage _returnvalue_4))
  (|PlayMontageandWaitProxy "None" _montage 1.0 "None" false 1.0 0.0 false
    (:then
      (Ability|Tasks|WaitGameplayEvent _montagetag 0
        (:EventReceived
          (bind _returnvalue_5 (Class|CombatInterface|GetCombatSocketLocation(Message) _returnvalue_2 _montagetag))
          (bind _outoverlappingactors (Class|AuraAbilitySystemLibrary|GetLivePlayersWithinRadius _returnvalue_2 (Utilities|Array|MakeArray _returnvalue_2) 45.0 _returnvalue_5))
          (for _array_element _outoverlappingactors
            (if (Class|AuraAbilitySystemLibrary|IsNotFriend (Ability|GetAvatarActorfromActorInfo) _array_element)
              (Class|AuraDamageGameplayAbility|CauseDamage _array_element))))))
    (:OnCompleted
      _)
    (:OnInterrupted
      _)
    (:OnCancelled
      _))
  (Class|GameplayAbility|ExecuteGameplayCuewithParams "(TagName=\"GameplayCue.MeeleeImpact\")" (Ability|GameplayCue|MakeGameplayCueParameters :AggregatedSourceTags (GameplayTags|MakeGameplayTagContainerfromTag _montagetag) :Location _returnvalue_5 :Normal (Transformation|GetActorLocation _array_element) :EffectCauser (Ability|GetAvatarActorfromActorInfo)))
  (Ability|EndAbility))

(fn GetRandomAttackMontage
  (params (Array :type Array%20of%20Tagged%20Montage%20Structures))
  (bind _output_get (Variables|Default|SetTaggedMontage (Class|AuraDamageGameplayAbility|GetRandomTaggedMontagefromArray Array)))
  (return (.Montage (Utilities|Struct|BreakTaggedMontage _output_get)) (.MontageTag (Utilities|Struct|BreakTaggedMontage _output_get)) (.ImpactSound (Utilities|Struct|BreakTaggedMontage _output_get))))