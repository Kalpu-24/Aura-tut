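; Enemy ranged attack gameplay ability that fires a projectile at the avatar's combat target.
; On activation it updates rotation motion warping toward the target through interface messages and plays a random tagged attack montage.
; When the montage's gameplay event tag arrives, it re-reads the target location and spawns the projectile from that montage's socket tag.
; The graph has no EndAbility call, and the montage is set not to stop when the ability ends.
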(event Ability|EventActivateAbility
  (bind _returnvalue (Ability|GetAvatarActorfromActorInfo))
  (bind _returnvalue_2 (Class|TargetInterface|GetCombatTarget(Message) _returnvalue))
  (Class|CombatInterface|UpdateRotationMotionWarp(Message) _returnvalue (Transformation|GetActorLocation _returnvalue_2))
  (bind _returnvalue_3 (Class|CombatInterface|GetAttackMontages(Message) _returnvalue))
  (bind (_montage _montagetag _sockettag) (CallFunction|GetRandomAttackMontage _returnvalue_3))
  (|PlayMontageandWaitProxy "None" _montage 1.0 "None" false 1.0 0.0 false
    (:then
      (Ability|Tasks|WaitGameplayEvent _montagetag 0 true
        (:EventReceived
          (bind _returnvalue_4 (Class|TargetInterface|GetCombatTarget(Message) (Ability|GetAvatarActorfromActorInfo)))
          (Class|AuraProjectileSpell|SpawnProjectile (Transformation|GetActorLocation _returnvalue_4) _sockettag))))))

(event Ability|EventOnEndAbility
  (params (bWasCancelled :type Boolean)))

(fn GetRandomAttackMontage
  (params (Array :type Array%20of%20Tagged%20Montage%20Structures))
  (bind _output_get (LocalVariables|SetTaggedMontage (Class|AuraDamageGameplayAbility|GetRandomTaggedMontagefromArray Array)))
  (return (.Montage (Utilities|Struct|BreakTaggedMontage _output_get)) (.MontageTag (Utilities|Struct|BreakTaggedMontage _output_get)) (.SocketTag (Utilities|Struct|BreakTaggedMontage _output_get)) (.ImpactSound (Utilities|Struct|BreakTaggedMontage _output_get))))