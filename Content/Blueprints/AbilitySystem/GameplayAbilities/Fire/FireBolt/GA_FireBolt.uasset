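; GA_FireBolt is a gameplay ability that casts a fire bolt toward the location under the mouse cursor.
; On activation it gets cursor target data, turns the avatar toward that point through a motion-warp rotation message and plays the cast montage.
; A montage gameplay event (Event.Montage.FireBolt) times the projectile spawn toward the stored target, after which the ability ends.
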(event Ability|EventActivateAbility
  (bind _datahandle (|TargetDataUnderMouse)
    (:ValidData
      (bind _output_get (Variables|Default|SetProjectileTargetLocation (.Location (Collision|BreakHitResult (Ability|TargetData|GetHitResultfromTargetData _datahandle)))))
      (Class|CombatInterface|UpdateRotationMotionWarp(Message) (Ability|GetAvatarActorfromActorInfo) _output_get)
      (|PlayMontageandWaitProxy "None" "/Game/Assets/Characters/Aura/Animations/Abilities/Cast_FireBolt_Montage.Cast_FireBolt_Montage" 1.0 "None" true 1.0 0.0 false
        (:then
          (Ability|Tasks|WaitGameplayEvent "(TagName=\"Event.Montage.FireBolt\")" 0
            (:EventReceived
              (Class|AuraProjectileSpell|SpawnFireBolt (Variables|Default|GetProjectileTargetLocation))
              (Ability|EndAbility))))))))

(event Ability|EventOnEndAbility
  (params (bWasCancelled :type Boolean)))